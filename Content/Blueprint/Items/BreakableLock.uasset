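; BreakableLock is an interactable lock actor for the downtown area that is removed once opened with the lock key.
; It reads DowntownLock from GI_Perso at BeginPlay and destroys itself if already unlocked, otherwise creates a P_Interact prompt widget.
; The Coll component's overlaps with the first-person character show and hide that prompt.
; Interact checks LockKey in the game instance, then clears DowntownLock and destroys the actor, so the unlock persists across level loads.
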(event `self.ReceiveBeginPlay`
  (bind _asgi_perso (cast `/Game/GameInstance/GI_Perso` (`GameplayStatics.GetGameInstance`)))
  (if (`/Game/GameInstance/GI_Perso.DowntownLock` _asgi_perso)
    (bind _returnvalue (`|CreateWidget` "/Game/Blueprint/Prompt/P_Interact.P_Interact_C"))
    (set `self.InteractPrompt` _returnvalue)
    (else
      (`self.K2_DestroyActor`))))

(event `/Game/Blueprint/BPI_Interact.Interact`
  (bind _asgi_perso (cast `/Game/GameInstance/GI_Perso` (`GameplayStatics.GetGameInstance`)))
  (if (`/Game/GameInstance/GI_Perso.LockKey` _asgi_perso)
    (set `/Game/GameInstance/GI_Perso.DowntownLock` false _asgi_perso)
    (`self.K2_DestroyActor`)))

(event `self.Coll.OnComponentBeginOverlap`
  (params (OverlappedComponent :type "PrimitiveComponent Object Reference") (OtherActor :type "Actor Object Reference") (OtherComp :type "PrimitiveComponent Object Reference") (OtherBodyIndex :type Integer) (bFromSweep :type Boolean) (SweepResult :type "HitResult Structure (by ref)"))
  (cast `/Game/FirstPerson/Blueprints/BP_FirstPersonCharacter` OtherActor)
  (`UserWidget.AddToViewport` (`self.InteractPrompt`) 0))

(event `self.Coll.OnComponentEndOverlap`
  (params (OverlappedComponent :type "PrimitiveComponent Object Reference") (OtherActor :type "Actor Object Reference") (OtherComp :type "PrimitiveComponent Object Reference") (OtherBodyIndex :type Integer))
  (cast `/Game/FirstPerson/Blueprints/BP_FirstPersonCharacter` OtherActor)
  (`Widget.RemoveFromParent` (`self.InteractPrompt`)))

(fn `UserConstructionScript`)