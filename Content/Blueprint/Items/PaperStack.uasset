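; Paper stack pickup that grants the player the blank paper item, recorded as the BlankPaper flag in GI_Perso.
; On BeginPlay it destroys itself if that flag is set, otherwise it creates the interact and obtained widgets.
; A sphere overlap shows or hides the prompt for the first-person character.
; Interact sets the flag, plays a sound, destroys the components and shows the obtained notice briefly, leaving the actor alive.
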(event `self.ReceiveBeginPlay`
  (bind _asgi_perso (cast `/Game/GameInstance/GI_Perso` (`GameplayStatics.GetGameInstance`)))
  (if (`/Game/GameInstance/GI_Perso.BlankPaper` _asgi_perso)
    (`self.K2_DestroyActor`)
    (else
      (bind _returnvalue (`|CreateWidget` "/Game/Blueprint/Prompt/P_Interact.P_Interact_C"))
      (set `self.InteractPrompt` _returnvalue)
      (bind _returnvalue_2 (`|CreateWidget` "/Game/Blueprint/Prompt/P_obtained_Blank_Paper.P_obtained_Blank_Paper_C"))
      (set `self.ObtainedPrompt` _returnvalue_2))))

(event `/Game/Blueprint/BPI_Interact.Interact`
  (bind _obtainedprompt (`self.ObtainedPrompt`))
  (bind _asgi_perso (cast `/Game/GameInstance/GI_Perso` (`GameplayStatics.GetGameInstance`)))
  (set `/Game/GameInstance/GI_Perso.BlankPaper` true _asgi_perso)
  (`GameplayStatics.PlaySound2D` "/Game/Blueprint/Items/DocumentsMissionDay1/PaperTake_Cue.PaperTake_Cue" 1.0 1.0 0.0 null null)
  (`UserWidget.AddToViewport` _obtainedprompt 0)
  (`ActorComponent.K2_DestroyComponent` (`self.Paper`))
  (`ActorComponent.K2_DestroyComponent` (`self.Sphere`))
  (`ActorComponent.K2_DestroyComponent` (`self.StaticMesh`))
  (`ActorComponent.K2_DestroyComponent` (`self.StaticMesh1`))
  (`KismetSystemLibrary.Delay` 3.0)
  (`Widget.RemoveFromParent` _obtainedprompt))

(event `self.Sphere.OnComponentBeginOverlap`
  (params (OverlappedComponent :type "PrimitiveComponent Object Reference") (OtherActor :type "Actor Object Reference") (OtherComp :type "PrimitiveComponent Object Reference") (OtherBodyIndex :type Integer) (bFromSweep :type Boolean) (SweepResult :type "HitResult Structure (by ref)"))
  (cast `/Game/FirstPerson/Blueprints/BP_FirstPersonCharacter` OtherActor)
  (`UserWidget.AddToViewport` (`self.InteractPrompt`) 0))

(event `self.Sphere.OnComponentEndOverlap`
  (params (OverlappedComponent :type "PrimitiveComponent Object Reference") (OtherActor :type "Actor Object Reference") (OtherComp :type "PrimitiveComponent Object Reference") (OtherBodyIndex :type Integer))
  (cast `/Game/FirstPerson/Blueprints/BP_FirstPersonCharacter` OtherActor)
  (`Widget.RemoveFromParent` (`self.InteractPrompt`)))

(fn `UserConstructionScript`)