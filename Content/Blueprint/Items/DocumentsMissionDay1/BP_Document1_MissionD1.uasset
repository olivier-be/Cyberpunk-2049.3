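; BP_Document1_MissionD1 is a collectible document for the Day 1 mission that opens as a newspaper when interacted with.
; Overlap with the first-person character toggles an interact-or-take prompt; interacting plays a sound, shows the newspaper widget and pauses the game.
; Taking it sets the GI_Perso flag, advances the mission counter, removes mesh and collision, and briefly shows an obtained notice.
; The actor destroys itself on BeginPlay if already collected.
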(event `self.ReceiveBeginPlay`
  (bind _asgi_perso (cast `/Game/GameInstance/GI_Perso` (`GameplayStatics.GetGameInstance`)))
  (if (== (`/Game/GameInstance/GI_Perso.Document1D1` _asgi_perso) 0)
    (bind _returnvalue (`|CreateWidget` "/Game/Blueprint/Prompt/P_Interact_or_take.P_Interact_or_take_C"))
    (set `self.InteractPrompt` _returnvalue)
    (bind _returnvalue_2 (`|CreateWidget` "/Game/Blueprint/Items/DocumentsMissionDay1/P_obtained_Document1.P_obtained_Document1_C"))
    (set `self.ObtainedPrompt` _returnvalue_2)
    (else
      (`self.K2_DestroyActor`))))

(event `self.Interact`
  (`GameplayStatics.PlaySound2D` "/Game/SoundAppartement/Notes_sound.Notes_sound" 1.0 1.0 0.0 null null)
  (bind _returnvalue (`|CreateWidget` "/Game/Blueprint/Note/WG_NewsPaper.WG_NewsPaper_C"))
  (`UserWidget.AddToViewport` _returnvalue 0)
  (set `PlayerController.bShowMouseCursor` true (`GameplayStatics.GetPlayerController` 0))
  (`GameplayStatics.SetGamePaused` true))

(event `/Game/Blueprint/BPI_Interact.TakeWhenChoiceObject`
  (bind _asgi_perso (cast `/Game/GameInstance/GI_Perso` (`GameplayStatics.GetGameInstance`)))
  (set `/Game/GameInstance/GI_Perso.Document1D1` 1 _asgi_perso)
  (bind _result (`/Engine/EditorBlueprintResources/StandardMacros.IncrementInt` (`/Game/GameInstance/GI_Perso.curMissionBalise` _asgi_perso))
    (:`  `
      (set `/Game/GameInstance/GI_Perso.curMissionBalise` _result _asgi_perso)
      (`GameplayStatics.PlaySoundAtLocation` "/Game/Blueprint/Items/DocumentsMissionDay1/PaperTake_Cue.PaperTake_Cue" (`self.K2_GetActorLocation`) (struct) 1.0 1.0 0.0 null null null null)
      (`UserWidget.AddToViewport` (`self.ObtainedPrompt`) 0)
      (`ActorComponent.K2_DestroyComponent` (`self.Coll`))
      (`ActorComponent.K2_DestroyComponent` (`self.Book`))
      (`KismetSystemLibrary.Delay` 3.0)
      (`Widget.RemoveFromParent` (`self.ObtainedPrompt`)))))

(event `self.Coll.OnComponentBeginOverlap`
  (params (OverlappedComponent :type "PrimitiveComponent Object Reference") (OtherActor :type "Actor Object Reference") (OtherComp :type "PrimitiveComponent Object Reference") (OtherBodyIndex :type Integer) (bFromSweep :type Boolean) (SweepResult :type "HitResult Structure (by ref)"))
  (cast `/Game/FirstPerson/Blueprints/BP_FirstPersonCharacter` OtherActor)
  (`UserWidget.AddToViewport` (`self.InteractPrompt`) 0))

(event `self.Coll.OnComponentEndOverlap`
  (params (OverlappedComponent :type "PrimitiveComponent Object Reference") (OtherActor :type "Actor Object Reference") (OtherComp :type "PrimitiveComponent Object Reference") (OtherBodyIndex :type Integer))
  (cast `/Game/FirstPerson/Blueprints/BP_FirstPersonCharacter` OtherActor)
  (`Widget.RemoveFromParent` (`self.InteractPrompt`)))

(fn `UserConstructionScript`)