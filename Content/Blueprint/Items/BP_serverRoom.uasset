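; Server room key pickup that stays in the level only when the game instance's CharacterDecision is high enough and it is not Day 1.
; Overlapping its sphere as the first-person character shows an interact prompt.
; Interact sets the ServerRoomKey flag on GI_Perso, plays a click and shows a timed "obtained" widget.
; It then destroys only the sphere and mesh, leaving the actor alive for the timer to remove that widget.
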(event `self.ReceiveBeginPlay`
  (bind _asgi_perso (cast `/Game/GameInstance/GI_Perso` (`GameplayStatics.GetGameInstance`)))
  (if (and (>= (`/Game/GameInstance/GI_Perso.character_decision` _asgi_perso) 0.6) (!= (`/Game/GameInstance/GI_Perso.day` _asgi_perso) 1))
    (bind _returnvalue (`|CreateWidget` "/Game/Blueprint/Prompt/P_Interact.P_Interact_C"))
    (set `self.InteractPrompt` _returnvalue)
    (bind _returnvalue_2 (`|CreateWidget` "/Game/Blueprint/Prompt/P_obtained_Server_Key.P_obtained_Server_Key_C"))
    (set `self.ObtainedPrompt` _returnvalue_2)
    (else
      (`self.K2_DestroyActor`))))

(event `self.Interact`
  (bind _asgi_perso (cast `/Game/GameInstance/GI_Perso` (`GameplayStatics.GetGameInstance`)))
  (set `/Game/GameInstance/GI_Perso.ServerRoomKey` true _asgi_perso)
  (`GameplayStatics.PlaySound2D` "/Engine/VREditor/Sounds/UI/Click_on_Button.Click_on_Button" 1.0 1.0 0.0 null null)
  (`UserWidget.AddToViewport` (`self.ObtainedPrompt`) 0)
  (`KismetSystemLibrary.K2_SetTimer` null "RemoveObtainedPrompt" 3.0)
  (`ActorComponent.K2_DestroyComponent` (`self.Sphere`))
  (`ActorComponent.K2_DestroyComponent` (`self.StaticMesh`)))

(event `self.Sphere.OnComponentBeginOverlap`
  (params (OverlappedComponent :type "PrimitiveComponent Object Reference") (OtherActor :type "Actor Object Reference") (OtherComp :type "PrimitiveComponent Object Reference") (OtherBodyIndex :type Integer) (bFromSweep :type Boolean) (SweepResult :type "HitResult Structure (by ref)"))
  (cast `/Game/FirstPerson/Blueprints/BP_FirstPersonCharacter` OtherActor)
  (`UserWidget.AddToViewport` (`self.InteractPrompt`) 0))

(event `self.Sphere.OnComponentEndOverlap`
  (params (OverlappedComponent :type "PrimitiveComponent Object Reference") (OtherActor :type "Actor Object Reference") (OtherComp :type "PrimitiveComponent Object Reference") (OtherBodyIndex :type Integer))
  (cast `/Game/FirstPerson/Blueprints/BP_FirstPersonCharacter` OtherActor)
  (`Widget.RemoveFromParent` (`self.InteractPrompt`)))

(fn `RemoveObtainedPrompt`
  (`Widget.RemoveFromParent` (`self.ObtainedPrompt`)))

(fn `UserConstructionScript`)