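; BP_Access_Key_LVL1 is a level 1 access card pickup that destroys itself on BeginPlay if the GameInstance already records it as owned.
; A sphere overlap shows an interact prompt to the first-person character.
; Interact sets the card flag, advances the mission marker index, plays a sound, shows timed feedback and removes the mesh and sphere.
; It then clears the objective in WBP_Main and, after a delay, sets the upstairs worklabs objective.
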(event `self.ReceiveBeginPlay`
  (bind _asgi_perso (cast `/Game/GameInstance/GI_Perso` (`GameplayStatics.GetGameInstance`)))
  (if (`/Game/GameInstance/GI_Perso.AccessCardLvL1` _asgi_perso)
    (`self.K2_DestroyActor`)
    (else
      (bind _returnvalue (`|CreateWidget` "/Game/Blueprint/Prompt/P_Interact.P_Interact_C"))
      (set `self.InteractPrompt` _returnvalue)
      (bind _returnvalue_2 (`|CreateWidget` "/Game/Blueprint/Prompt/P_obtained_Access_Card_Lvl1.P_obtained_Access_Card_Lvl1_C"))
      (set `self.ObtainedPrompt` _returnvalue_2))))

(event `/Game/Blueprint/BPI_Interact.Interact`
  (bind _asgi_perso (cast `/Game/GameInstance/GI_Perso` (`GameplayStatics.GetGameInstance`)))
  (bind _result (`/Engine/EditorBlueprintResources/StandardMacros.IncrementInt` (`/Game/GameInstance/GI_Perso.curMissionBalise` _asgi_perso))
    (:`  `
      (set `/Game/GameInstance/GI_Perso.curMissionBalise` _result _asgi_perso)
      (set `/Game/GameInstance/GI_Perso.AccessCardLvL1` true _asgi_perso)
      (`GameplayStatics.PlaySound2D` "/Engine/VREditor/Sounds/UI/Click_on_Button.Click_on_Button" 1.0 1.0 0.0 null null)
      (`UserWidget.AddToViewport` (`self.ObtainedPrompt`) 0)
      (`KismetSystemLibrary.K2_SetTimer` null "RemoveObtainedPrompt" 3.0)
      (`ActorComponent.K2_DestroyComponent` (`self.Sphere`))
      (`ActorComponent.K2_DestroyComponent` (`self.StaticMesh`))
      (bind _returnvalue (`|CreateWidget` "/Game/Dialogue/Day1/P_GoUpstair.P_GoUpstair_C"))
      (`UserWidget.AddToViewport` _returnvalue 0)
      (bind _asgi_perso_2 (cast `/Game/GameInstance/GI_Perso` (`GameplayStatics.GetGameInstance`)))
      (bind _output_get (set `/Game/GameInstance/GI_Perso.CurrentObjective` "" _asgi_perso_2))
      (bind _foundwidgets (`WidgetBlueprintLibrary.GetAllWidgetsOfClass` "/Game/HUD/WBP_Main.WBP_Main_C" false))
      (for _array_element _foundwidgets
        (`/Game/HUD/WBP_Main.UpdateMissionPrompt` _array_element _output_get)
        (`KismetSystemLibrary.Delay` 5.0)
        (bind _output_get_2 (set `/Game/GameInstance/GI_Perso.CurrentObjective` "Go to the upstairs worklabs" _asgi_perso_2))
        (bind _foundwidgets_2 (`WidgetBlueprintLibrary.GetAllWidgetsOfClass` "/Game/HUD/WBP_Main.WBP_Main_C" false))
        (for _array_element_2 _foundwidgets_2
          (`/Game/HUD/WBP_Main.UpdateMissionPrompt` _array_element_2 _output_get_2))))))

(event `self.Sphere.OnComponentBeginOverlap`
  (params (OverlappedComponent :type "PrimitiveComponent Object Reference") (OtherActor :type "Actor Object Reference") (OtherComp :type "PrimitiveComponent Object Reference") (OtherBodyIndex :type Integer) (bFromSweep :type Boolean) (SweepResult :type "HitResult Structure (by ref)"))
  (cast `/Game/FirstPerson/Blueprints/BP_FirstPersonCharacter` OtherActor)
  (`UserWidget.AddToViewport` (`self.InteractPrompt`) 0))

(event `self.Sphere.OnComponentEndOverlap`
  (params (OverlappedComponent :type "PrimitiveComponent Object Reference") (OtherActor :type "Actor Object Reference") (OtherComp :type "PrimitiveComponent Object Reference") (OtherBodyIndex :type Integer))
  (cast `/Game/FirstPerson/Blueprints/BP_FirstPersonCharacter` OtherActor)
  (`Widget.RemoveFromParent` (`self.InteractPrompt`)))

(fn `RemoveObtainedPrompt`
  (`Widget.RemoveFromParent` (`self.ObtainedPrompt`)))

(fn `UserConstructionScript`)