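; BP_LockKey is a pickup key item that the first-person character collects through an Interact event.
; Overlapping its collision shows an interact prompt, and leaving hides it.
; Interact sets the LockKey flag on the GI_Perso game instance, plays a sound, destroys the key's components and shows an obtained prompt until a timer removes it.
; On BeginPlay the actor destroys itself if that flag is already set, so a collected key stays gone.
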(event `self.ReceiveBeginPlay`
  (bind _asgi_perso (cast `/Game/GameInstance/GI_Perso` (`GameplayStatics.GetGameInstance`)))
  (if (`/Game/GameInstance/GI_Perso.LockKey` _asgi_perso)
    (`self.K2_DestroyActor`)
    (else
      (bind _returnvalue (`|CreateWidget` "/Game/Blueprint/Prompt/P_Interact.P_Interact_C"))
      (set `self.InteractPrompt` _returnvalue)
      (bind _returnvalue_2 (`|CreateWidget` "/Game/Blueprint/Prompt/P_obtained_Lock_Keys.P_obtained_Lock_Keys_C"))
      (set `self.ObtainedPrompt` _returnvalue_2))))

(event `self.Interact`
  (bind _asgi_perso (cast `/Game/GameInstance/GI_Perso` (`GameplayStatics.GetGameInstance`)))
  (set `/Game/GameInstance/GI_Perso.LockKey` true _asgi_perso)
  (`GameplayStatics.PlaySoundAtLocation` "/Game/SoundAppartement/GetKeys_Cue.GetKeys_Cue" (0.0 0.0 0.0) (struct) 1.0 1.0 0.0 null null null null)
  (`UserWidget.AddToViewport` (`self.ObtainedPrompt`) 0)
  (`KismetSystemLibrary.K2_SetTimer` null "RemoveObtainedPrompt" 3.0)
  (`ActorComponent.K2_DestroyComponent` (`self.Key`))
  (`ActorComponent.K2_DestroyComponent` (`self.Coll`))
  (`ActorComponent.K2_DestroyComponent` (`self.Tag`)))

(event `self.Coll.OnComponentBeginOverlap`
  (params (OverlappedComponent :type "PrimitiveComponent Object Reference") (OtherActor :type "Actor Object Reference") (OtherComp :type "PrimitiveComponent Object Reference") (OtherBodyIndex :type Integer) (bFromSweep :type Boolean) (SweepResult :type "HitResult Structure (by ref)"))
  (cast `/Game/FirstPerson/Blueprints/BP_FirstPersonCharacter` OtherActor)
  (`UserWidget.AddToViewport` (`self.InteractPrompt`) 0))

(event `self.Coll.OnComponentEndOverlap`
  (params (OverlappedComponent :type "PrimitiveComponent Object Reference") (OtherActor :type "Actor Object Reference") (OtherComp :type "PrimitiveComponent Object Reference") (OtherBodyIndex :type Integer))
  (cast `/Game/FirstPerson/Blueprints/BP_FirstPersonCharacter` OtherActor)
  (`Widget.RemoveFromParent` (`self.InteractPrompt`)))

(fn `RemoveObtainedPrompt`
  (`Widget.RemoveFromParent` (`self.ObtainedPrompt`)))

(fn `UserConstructionScript`)