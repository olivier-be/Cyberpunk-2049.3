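; USB key pickup item that the player collects once, with its state stored in the GI_Perso game instance.
; On BeginPlay it destroys itself if the key is already owned, otherwise it creates an interact prompt widget.
; A sphere overlap with the first-person character shows or hides that prompt.
; Interact sets the flag, removes the mesh and sphere, and shows an "obtained" widget for a few seconds.
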(event `self.ReceiveBeginPlay`
  (bind _asgi_perso (cast `/Game/GameInstance/GI_Perso` (`GameplayStatics.GetGameInstance`)))
  (if (`/Game/GameInstance/GI_Perso.USBKey` _asgi_perso)
    (`self.K2_DestroyActor`)
    (else
      (bind _returnvalue (`|CreateWidget` "/Game/Blueprint/Prompt/P_Interact.P_Interact_C"))
      (set `self.InteractPrompt` _returnvalue))))

(event `/Game/Blueprint/BPI_Interact.Interact`
  (bind _asgi_perso (cast `/Game/GameInstance/GI_Perso` (`GameplayStatics.GetGameInstance`)))
  (set `/Game/GameInstance/GI_Perso.USBKey` true _asgi_perso)
  (bind _returnvalue (`|CreateWidget` "/Game/Blueprint/Prompt/P_obtained_USB_Key.P_obtained_USB_Key_C"))
  (`UserWidget.AddToViewport` _returnvalue 0)
  (`ActorComponent.K2_DestroyComponent` (`self.StaticMesh`))
  (`ActorComponent.K2_DestroyComponent` (`self.Sphere`))
  (`KismetSystemLibrary.Delay` 3.0)
  (`Widget.RemoveFromParent` _returnvalue)
  (`Widget.RemoveFromParent` (`self.InteractPrompt`)))

(event `self.Sphere.OnComponentBeginOverlap`
  (params (OverlappedComponent :type "PrimitiveComponent Object Reference") (OtherActor :type "Actor Object Reference") (OtherComp :type "PrimitiveComponent Object Reference") (OtherBodyIndex :type Integer) (bFromSweep :type Boolean) (SweepResult :type "HitResult Structure (by ref)"))
  (cast `/Game/FirstPerson/Blueprints/BP_FirstPersonCharacter` OtherActor)
  (`UserWidget.AddToViewport` (`self.InteractPrompt`) 0))

(event `self.Sphere.OnComponentEndOverlap`
  (params (OverlappedComponent :type "PrimitiveComponent Object Reference") (OtherActor :type "Actor Object Reference") (OtherComp :type "PrimitiveComponent Object Reference") (OtherBodyIndex :type Integer))
  (cast `/Game/FirstPerson/Blueprints/BP_FirstPersonCharacter` OtherActor)
  (`Widget.RemoveFromParent` (`self.InteractPrompt`)))

(fn `UserConstructionScript`)