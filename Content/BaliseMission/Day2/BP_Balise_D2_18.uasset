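; Day 2 mission beacon (balise) that puts the player to sleep and moves the game on to Day 3.
; It destroys itself outside Day 2, otherwise polls GI_Perso on Tick and activates when day and mission number match.
; While active, its sphere overlap toggles an interact prompt.
; Interacting advances the game instance state, while a delayed sequence shows a black screen with sound, clears the objective and displays Day 3 intro and dialogue widgets.
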(event `self.ReceiveBeginPlay`
  (bind _asgi_perso (cast `/Game/GameInstance/GI_Perso` (`GameplayStatics.GetGameInstance`)))
  (if (== (`/Game/GameInstance/GI_Perso.day` _asgi_perso) 2)
    (bind _returnvalue (`|CreateWidget` "/Game/Blueprint/Prompt/P_Interact.P_Interact_C"))
    (set `self.InteractPrompt` _returnvalue)
    (bind _returnvalue_2 (`|CreateWidget` "/Game/Blueprint/Prompt/BlackScreenSleep.BlackScreenSleep_C"))
    (set `self.BlackScreen` _returnvalue_2)
    (else
      (`self.K2_DestroyActor`))))

(event `self.ReceiveTick`
  (params (DeltaSeconds :type "Float (single-precision)"))
  (bind _asgi_perso (cast `/Game/GameInstance/GI_Perso` (`GameplayStatics.GetGameInstance`)))
  (if (and (== (`self.IsActive`) false) (and (== (`/Game/GameInstance/GI_Perso.day` _asgi_perso) (`self.Day`)) (== (`/Game/GameInstance/GI_Perso.curMissionBalise` _asgi_perso) (`self.MissionNb`))))
    (set `self.IsActive` true)
    (`self.ActivateBalise`)))

(event `self.Sphere.OnComponentBeginOverlap`
  (params (OverlappedComponent :type "PrimitiveComponent Object Reference") (OtherActor :type "Actor Object Reference") (OtherComp :type "PrimitiveComponent Object Reference") (OtherBodyIndex :type Integer) (bFromSweep :type Boolean) (SweepResult :type "HitResult Structure (by ref)"))
  (if (`self.IsActive`)
    (cast `/Game/FirstPerson/Blueprints/BP_FirstPersonCharacter` OtherActor)
    (`UserWidget.AddToViewport` (`self.InteractPrompt`) 0)))

(event `self.Sphere.OnComponentEndOverlap`
  (params (OverlappedComponent :type "PrimitiveComponent Object Reference") (OtherActor :type "Actor Object Reference") (OtherComp :type "PrimitiveComponent Object Reference") (OtherBodyIndex :type Integer))
  (if (`self.IsActive`)
    (cast `/Game/FirstPerson/Blueprints/BP_FirstPersonCharacter` OtherActor)
    (`Widget.RemoveFromParent` (`self.InteractPrompt`))))

(event `self.Interact`
  (if (`self.IsActive`)
    (`Widget.RemoveFromParent` (`self.InteractPrompt`))
    (`self.Sleep`)
    (bind _asgi_perso (cast `/Game/GameInstance/GI_Perso` (`GameplayStatics.GetGameInstance`)))
    (set `/Game/GameInstance/GI_Perso.day` 3 _asgi_perso)
    (set `/Game/GameInstance/GI_Perso.curMissionBalise` 1 _asgi_perso)
    (set `self.IsActive` false)))

(event `Sleep`
  (bind _blackscreen (`self.BlackScreen`))
  (`UserWidget.AddToViewport` _blackscreen 0)
  (`KismetSystemLibrary.Delay` 1.0)
  (`GameplayStatics.PlaySound2D` "/Game/SoundAppartement/SleepingSound_Cue.SleepingSound_Cue" 1.0 1.0 0.0 null null)
  (`KismetSystemLibrary.Delay` 3.0)
  (`Widget.RemoveFromParent` _blackscreen)
  (bind _asgi_perso (cast `/Game/GameInstance/GI_Perso` (`GameplayStatics.GetGameInstance`)))
  (bind _output_get (set `/Game/GameInstance/GI_Perso.CurrentObjective` "" _asgi_perso))
  (bind _foundwidgets (`WidgetBlueprintLibrary.GetAllWidgetsOfClass` "/Game/HUD/WBP_Main.WBP_Main_C" false))
  (for _array_element _foundwidgets
    (`/Game/HUD/WBP_Main.UpdateMissionPrompt` _array_element _output_get)
    (`KismetSystemLibrary.Delay` 2.0)
    (bind _returnvalue (`|CreateWidget` "/Game/Dialogue/Day3/P_Day3Intro.P_Day3Intro_C"))
    (`UserWidget.AddToViewport` _returnvalue 0)
    (`KismetSystemLibrary.Delay` 4.0)
    (bind _returnvalue_2 (`|CreateWidget` "/Game/Dialogue/Day3/P_DialogueWakeD3.P_DialogueWakeD3_C"))
    (`UserWidget.AddToViewport` _returnvalue_2 0)))

(fn `UserConstructionScript`)