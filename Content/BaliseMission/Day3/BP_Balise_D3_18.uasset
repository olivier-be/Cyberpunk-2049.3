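; Mission beacon for Day 3 (BP_Balise_D3_18) that triggers a scripted blackout sequence ending in a return to the main menu.
; It destroys itself on other days, and Tick activates it when GI_Perso's day and current mission match its own.
; When the first-person character enters its sphere, it shows the BlackScreenSleep widget, plays timed footstep, machine-gun and falling sounds via delays, then opens MainMenu.
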(event `self.ReceiveBeginPlay`
  (bind _asgi_perso (cast `/Game/GameInstance/GI_Perso` (`GameplayStatics.GetGameInstance`)))
  (if (== (`/Game/GameInstance/GI_Perso.day` _asgi_perso) 3)
    (bind _returnvalue (`|CreateWidget` "/Game/Blueprint/Prompt/BlackScreenSleep.BlackScreenSleep_C"))
    (set `self.BlackScreen` _returnvalue)
    (else
      (`self.K2_DestroyActor`))))

(event `self.ReceiveTick`
  (params (DeltaSeconds :type "Float (single-precision)"))
  (bind _asgi_perso (cast `/Game/GameInstance/GI_Perso` (`GameplayStatics.GetGameInstance`)))
  (if (and (== (`self.IsActive`) false) (and (== (`/Game/GameInstance/GI_Perso.day` _asgi_perso) (`self.Day`)) (== (`/Game/GameInstance/GI_Perso.curMissionBalise` _asgi_perso) (`self.MissionNb`))))
    (set `self.IsActive` true)
    (`self.ActivateBalise`)))

(event `self.Sphere.OnComponentBeginOverlap`
  (params (OverlappedComponent :type "PrimitiveComponent Object Reference") (OtherActor :type "Actor Object Reference") (OtherComp :type "PrimitiveComponent Object Reference") (OtherBodyIndex :type Integer) (bFromSweep :type Boolean) (SweepResult :type "HitResult Structure (by ref)"))
  (cast `/Game/FirstPerson/Blueprints/BP_FirstPersonCharacter` OtherActor)
  (if (`self.IsActive`)
    (`ActorComponent.K2_DestroyComponent` (`self.Sphere`))
    (cast `/Game/GameInstance/GI_Perso` (`GameplayStatics.GetGameInstance`))
    (`UserWidget.AddToViewport` (`self.BlackScreen`) 0)
    (set `self.IsActive` false)
    (`GameplayStatics.PlaySound2D` "/Game/SoundGlobal/Footsteps/FootstepSound.FootstepSound" 1.0 1.0 0.0 null null)
    (`KismetSystemLibrary.Delay` 1.0)
    (`GameplayStatics.PlaySound2D` "/Game/SoundGlobal/Footsteps/FootstepSound.FootstepSound" 1.0 1.0 0.0 null null)
    (`KismetSystemLibrary.Delay` 1.0)
    (`GameplayStatics.PlaySound2D` "/Game/SoundGlobal/Footsteps/FootstepSound.FootstepSound" 1.0 1.0 0.0 null null)
    (`KismetSystemLibrary.Delay` 1.0)
    (`GameplayStatics.PlaySound2D` "/Game/SoundGlobal/Footsteps/FootstepSound.FootstepSound" 1.0 1.0 0.0 null null)
    (`KismetSystemLibrary.Delay` 1.0)
    (`GameplayStatics.PlaySound2D` "/Game/SoundGlobal/dennish18-machine-gun-129928_Cue.dennish18-machine-gun-129928_Cue" 1.0 1.0 0.0 null null)
    (`KismetSystemLibrary.Delay` 3.0)
    (`GameplayStatics.PlaySound2D` "/Game/SoundGlobal/universfield-falling-259680_Cue.universfield-falling-259680_Cue" 1.0 1.0 0.0 null null)
    (`KismetSystemLibrary.Delay` 3.0)
    (`GameplayStatics.OpenLevel` "MainMenu")))

(fn `UserConstructionScript`)