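; Day 3 mission beacon (balise) that serves as an ending choice between stabilizing and destruction, and destroys itself on other days.
; Tick activates it when the day and current beacon mission in GI_Perso match its own.
; Its sphere overlap shows a stabilize prompt, or an interact-or-USB prompt if the player holds the USB key.
; Interact or TakewhenChoiceObject permanently disables it and runs the timed Stabilize or Explode sound and widget sequence.
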(event `self.ReceiveBeginPlay`
  (bind _asgi_perso (cast `/Game/GameInstance/GI_Perso` (`GameplayStatics.GetGameInstance`)))
  (if (== (`/Game/GameInstance/GI_Perso.day` _asgi_perso) 3)
    (bind _returnvalue (`|CreateWidget` "/Game/Blueprint/Prompt/P_stabilise.P_stabilise_C"))
    (set `self.InteractPrompt` _returnvalue)
    (bind _returnvalue_2 (`|CreateWidget` "/Game/Blueprint/Prompt/P_Interact_or_USB.P_Interact_or_USB_C"))
    (set `self.InteractUsb` _returnvalue_2)
    (else
      (`self.K2_DestroyActor`))))

(event `self.ReceiveTick`
  (params (DeltaSeconds :type "Float (single-precision)"))
  (if (not (`self.ForeverDeactivate`))
    (bind _asgi_perso (cast `/Game/GameInstance/GI_Perso` (`GameplayStatics.GetGameInstance`)))
    (if (and (== (`self.IsActive`) false) (and (== (`/Game/GameInstance/GI_Perso.day` _asgi_perso) (`self.Day`)) (== (`/Game/GameInstance/GI_Perso.curMissionBalise` _asgi_perso) (`self.MissionNb`))))
      (set `self.IsActive` true)
      (`self.ActivateBalise`))))

(event `self.Sphere.OnComponentBeginOverlap`
  (params (OverlappedComponent :type "PrimitiveComponent Object Reference") (OtherActor :type "Actor Object Reference") (OtherComp :type "PrimitiveComponent Object Reference") (OtherBodyIndex :type Integer) (bFromSweep :type Boolean) (SweepResult :type "HitResult Structure (by ref)"))
  (cast `/Game/FirstPerson/Blueprints/BP_FirstPersonCharacter` OtherActor)
  (if (`self.IsActive`)
    (bind _asgi_perso (cast `/Game/GameInstance/GI_Perso` (`GameplayStatics.GetGameInstance`)))
    (if (`/Game/GameInstance/GI_Perso.USBKey` _asgi_perso)
      (`UserWidget.AddToViewport` (`self.InteractUsb`) 0)
      (else
        (`UserWidget.AddToViewport` (`self.InteractPrompt`) 0)))))

(event `self.Sphere.OnComponentEndOverlap`
  (params (OverlappedComponent :type "PrimitiveComponent Object Reference") (OtherActor :type "Actor Object Reference") (OtherComp :type "PrimitiveComponent Object Reference") (OtherBodyIndex :type Integer))
  (cast `/Game/FirstPerson/Blueprints/BP_FirstPersonCharacter` OtherActor)
  (if (`self.IsActive`)
    (cast `/Game/GameInstance/GI_Perso` (`GameplayStatics.GetGameInstance`))
    (if (`/Game/GameInstance/GI_Perso.USBKey` (stale `self.Sphere.OnComponentBeginOverlap` _asgi_perso))
      (`Widget.RemoveFromParent` (`self.InteractUsb`))
      (else
        (`Widget.RemoveFromParent` (`self.InteractPrompt`))))))

(event `self.Interact`
  (if (`self.IsActive`)
    (set `self.IsActive` false)
    (set `self.ForeverDeactivate` true)
    (`Widget.RemoveFromParent` (`self.InteractPrompt`))
    (`Widget.RemoveFromParent` (`self.InteractUsb`))
    (`self.Stabilize`)))

(event `/Game/Blueprint/BPI_Interact.TakeWhenChoiceObject`
  (if (`self.IsActive`)
    (set `self.IsActive` false)
    (set `self.ForeverDeactivate` true)
    (`Widget.RemoveFromParent` (`self.InteractPrompt`))
    (`Widget.RemoveFromParent` (`self.InteractUsb`))
    (`self.Explode`)))

(event `Explode`
  (bind _returnvalue (`self.K2_GetActorLocation`))
  (bind _asgi_perso (cast `/Game/GameInstance/GI_Perso` (`GameplayStatics.GetGameInstance`)))
  (`GameplayStatics.PlaySound2D` "/Engine/VREditor/Sounds/UI/Object_Snaps_To_Another_Actor.Object_Snaps_To_Another_Actor" 1.0 1.0 0.0 null null)
  (`KismetSystemLibrary.Delay` 2.0)
  (`GameplayStatics.PlaySoundAtLocation` "/Game/SoundGlobal/ChargeBeforeExp.ChargeBeforeExp" _returnvalue (struct) 1.0 1.0 0.0 null null null null)
  (`KismetSystemLibrary.Delay` 6.0)
  (bind _returnvalue_2 (`|CreateWidget` "/Game/Dialogue/Day3/P_Destruction_1.P_Destruction_1_C"))
  (`UserWidget.AddToViewport` _returnvalue_2 0)
  (`KismetSystemLibrary.Delay` 5.0)
  (set `/Game/GameInstance/GI_Perso.explosion` true _asgi_perso)
  (`GameplayStatics.PlaySound2D` "/Game/SoundGlobal/Sing_for_Absolution_Cue.Sing_for_Absolution_Cue" 1.0 1.0 0.0 null null)
  (`KismetSystemLibrary.Delay` 2.0)
  (`GameplayStatics.PlaySoundAtLocation` "/Game/SoundGlobal/short_circuit_Cue.short_circuit_Cue" _returnvalue (struct) 1.0 1.0 0.0 null null null null)
  (`GameplayStatics.PlaySound2D` "/Game/SoundGlobal/Alarm_Cue.Alarm_Cue" 1.0 1.0 0.0 null null)
  (`KismetSystemLibrary.Delay` 3.0)
  (bind _returnvalue_3 (`|CreateWidget` "/Game/Dialogue/Day3/DestructionFinal.DestructionFinal_C"))
  (`UserWidget.AddToViewport` _returnvalue_3 0))

(event `Stabilize`
  (cast `/Game/GameInstance/GI_Perso` (`GameplayStatics.GetGameInstance`))
  (`GameplayStatics.PlaySound2D` "/Engine/VREditor/Sounds/UI/Object_Snaps_To_Another_Actor.Object_Snaps_To_Another_Actor" 1.0 1.0 0.0 null null)
  (`KismetSystemLibrary.Delay` 2.0)
  (`GameplayStatics.PlaySoundAtLocation` "/Game/SoundGlobal/ChargeBeforeExp.ChargeBeforeExp" (`self.K2_GetActorLocation`) (struct) 1.0 1.0 0.0 null null null null)
  (`KismetSystemLibrary.Delay` 6.0)
  (bind _returnvalue (`|CreateWidget` "/Game/Dialogue/Day3/StabilizeFinal.StabilizeFinal_C"))
  (`UserWidget.AddToViewport` _returnvalue 0))

(fn `UserConstructionScript`)