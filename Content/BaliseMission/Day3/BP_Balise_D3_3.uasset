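; Day 3 mission beacon that marks the player entering the lab and advances the objective to taking the access card.
; It removes itself on other days and polls GI_Perso each tick, activating when day and mission index match.
; Player overlap while active destroys the trigger sphere, shows the lab-entry widget and clears the objective.
; After a delay it pushes the new objective to WBP_Main, increments the mission index and deactivates.
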(event `self.ReceiveBeginPlay`
  (bind _asgi_perso (cast `/Game/GameInstance/GI_Perso` (`GameplayStatics.GetGameInstance`)))
  (if (not (== (`/Game/GameInstance/GI_Perso.day` _asgi_perso) 3))
    (`self.K2_DestroyActor`)))

(event `self.ReceiveTick`
  (params (DeltaSeconds :type "Float (single-precision)"))
  (bind _asgi_perso (cast `/Game/GameInstance/GI_Perso` (`GameplayStatics.GetGameInstance`)))
  (if (and (== (`self.IsActive`) false) (and (== (`/Game/GameInstance/GI_Perso.day` _asgi_perso) (`self.Day`)) (== (`/Game/GameInstance/GI_Perso.curMissionBalise` _asgi_perso) (`self.MissionNb`))))
    (set `self.IsActive` true)
    (`self.ActivateBalise`)))

(event `self.Sphere.OnComponentBeginOverlap`
  (params (OverlappedComponent :type "PrimitiveComponent Object Reference") (OtherActor :type "Actor Object Reference") (OtherComp :type "PrimitiveComponent Object Reference") (OtherBodyIndex :type Integer) (bFromSweep :type Boolean) (SweepResult :type "HitResult Structure (by ref)"))
  (cast `/Game/FirstPerson/Blueprints/BP_FirstPersonCharacter` OtherActor)
  (if (`self.IsActive`)
    (`ActorComponent.K2_DestroyComponent` (`self.Sphere`))
    (bind _asgi_perso (cast `/Game/GameInstance/GI_Perso` (`GameplayStatics.GetGameInstance`)))
    (bind _returnvalue (`|CreateWidget` "/Game/Dialogue/Day3/P_EnteredLabD3.P_EnteredLabD3_C"))
    (`UserWidget.AddToViewport` _returnvalue 0)
    (bind _asgi_perso_2 (cast `/Game/GameInstance/GI_Perso` (`GameplayStatics.GetGameInstance`)))
    (bind _output_get (set `/Game/GameInstance/GI_Perso.CurrentObjective` "" _asgi_perso_2))
    (bind _foundwidgets (`WidgetBlueprintLibrary.GetAllWidgetsOfClass` "/Game/HUD/WBP_Main.WBP_Main_C" false))
    (for _array_element _foundwidgets
      (`/Game/HUD/WBP_Main.UpdateMissionPrompt` _array_element _output_get)
      (`KismetSystemLibrary.Delay` 12.0)
      (bind _output_get_2 (set `/Game/GameInstance/GI_Perso.CurrentObjective` "Take your access card" _asgi_perso_2))
      (bind _foundwidgets_2 (`WidgetBlueprintLibrary.GetAllWidgetsOfClass` "/Game/HUD/WBP_Main.WBP_Main_C" false))
      (for _array_element_2 _foundwidgets_2
        (`/Game/HUD/WBP_Main.UpdateMissionPrompt` _array_element_2 _output_get_2)
        (bind _result (`/Engine/EditorBlueprintResources/StandardMacros.IncrementInt` (`/Game/GameInstance/GI_Perso.curMissionBalise` _asgi_perso))
          (:`  `
            (set `/Game/GameInstance/GI_Perso.curMissionBalise` _result _asgi_perso)
            (set `self.IsActive` false)))))))

(fn `UserConstructionScript`)