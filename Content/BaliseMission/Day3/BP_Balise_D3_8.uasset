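; BP_Balise_D3_8 is a mission beacon (balise) for Day 3 that destroys itself at BeginPlay on any other day.
; Tick polls GI_Perso and calls ActivateBalise once the day and current beacon index match its Day and MissionNb.
; When BP_FirstPersonCharacter overlaps the Sphere while it is active, it deactivates permanently and increments CurMissionBalise, advancing the beacon sequence.
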(event `self.ReceiveBeginPlay`
  (bind _asgi_perso (cast `/Game/GameInstance/GI_Perso` (`GameplayStatics.GetGameInstance`)))
  (if (not (== (`/Game/GameInstance/GI_Perso.day` _asgi_perso) 3))
    (`self.K2_DestroyActor`)))

(event `self.ReceiveTick`
  (params (DeltaSeconds :type "Float (single-precision)"))
  (if (not (`self.ForeverDeactivate`))
    (bind _asgi_perso (cast `/Game/GameInstance/GI_Perso` (`GameplayStatics.GetGameInstance`)))
    (if (and (== (`self.IsActive`) false) (and (== (`/Game/GameInstance/GI_Perso.day` _asgi_perso) (`self.Day`)) (== (`/Game/GameInstance/GI_Perso.curMissionBalise` _asgi_perso) (`self.MissionNb`))))
      (set `self.IsActive` true)
      (`self.ActivateBalise`))))

(event `self.Sphere.OnComponentBeginOverlap`
  (params (OverlappedComponent :type "PrimitiveComponent Object Reference") (OtherActor :type "Actor Object Reference") (OtherComp :type "PrimitiveComponent Object Reference") (OtherBodyIndex :type Integer) (bFromSweep :type Boolean) (SweepResult :type "HitResult Structure (by ref)"))
  (cast `/Game/FirstPerson/Blueprints/BP_FirstPersonCharacter` OtherActor)
  (if (`self.IsActive`)
    (set `self.IsActive` false)
    (set `self.ForeverDeactivate` true)
    (bind _asgi_perso (cast `/Game/GameInstance/GI_Perso` (`GameplayStatics.GetGameInstance`)))
    (bind _result (`/Engine/EditorBlueprintResources/StandardMacros.IncrementInt` (`/Game/GameInstance/GI_Perso.curMissionBalise` _asgi_perso))
      (:`  `
        (set `/Game/GameInstance/GI_Perso.curMissionBalise` _result _asgi_perso)))))

(fn `UserConstructionScript`)