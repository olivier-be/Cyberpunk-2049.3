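; Mission beacon (balise) for Day 1 where the player places a document, revealing a hidden book.
; Tick activates it when the game instance's day and current mission match its own, and sphere overlap toggles a place-or-steal prompt.
; Interact advances the document state, shows the book with a paper sound, then permanently deactivates the beacon and increments the mission counter.
; TakewhenChoiceObject jumps straight to that completion step without revealing the book.
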(event `self.ReceiveBeginPlay`
  (bind _returnvalue (`|CreateWidget` "/Game/Blueprint/Prompt/P_Place_or_steal.P_Place_or_steal_C"))
  (set `self.InteractPrompt` _returnvalue)
  (`SceneComponent.SetHiddenInGame` (`self.book`) true false))

(event `self.ReceiveTick`
  (params (DeltaSeconds :type "Float (single-precision)"))
  (if (not (`self.ForeverDeactivate`))
    (bind _asgi_perso (cast `/Game/GameInstance/GI_Perso` (`GameplayStatics.GetGameInstance`)))
    (if (and (== (`self.IsActive`) false) (and (== (`/Game/GameInstance/GI_Perso.day` _asgi_perso) (`self.Day`)) (== (`/Game/GameInstance/GI_Perso.curMissionBalise` _asgi_perso) (`self.MissionNb`))))
      (set `self.IsActive` true)
      (`self.ActivateBalise`))))

(event `self.Sphere.OnComponentBeginOverlap`
  (params (OverlappedComponent :type "PrimitiveComponent Object Reference") (OtherActor :type "Actor Object Reference") (OtherComp :type "PrimitiveComponent Object Reference") (OtherBodyIndex :type Integer) (bFromSweep :type Boolean) (SweepResult :type "HitResult Structure (by ref)"))
  (cast `/Game/FirstPerson/Blueprints/BP_FirstPersonCharacter` OtherActor)
  (if (`self.IsActive`)
    (`UserWidget.AddToViewport` (`self.InteractPrompt`) 0)))

(event `self.Sphere.OnComponentEndOverlap`
  (params (OverlappedComponent :type "PrimitiveComponent Object Reference") (OtherActor :type "Actor Object Reference") (OtherComp :type "PrimitiveComponent Object Reference") (OtherBodyIndex :type Integer))
  (cast `/Game/FirstPerson/Blueprints/BP_FirstPersonCharacter` OtherActor)
  (if (`self.IsActive`)
    (`Widget.RemoveFromParent` (`self.InteractPrompt`))))

(event `/Game/Blueprint/BPI_Interact.Interact`
  (bind _asgi_perso (cast `/Game/GameInstance/GI_Perso` (`GameplayStatics.GetGameInstance`)))
  (if (== (`/Game/GameInstance/GI_Perso.Document1D1` _asgi_perso) 1)
    (set `/Game/GameInstance/GI_Perso.Document1D1` 2 _asgi_perso)
    (`SceneComponent.SetHiddenInGame` (`self.book`) false false)
    (`GameplayStatics.PlaySound2D` "/Game/Blueprint/Items/DocumentsMissionDay1/PaperTake_Cue.PaperTake_Cue" 1.0 1.0 0.0 null null)
    (if (`self.IsActive`) :!label _label
      (set `self.IsActive` false)
      (set `self.ForeverDeactivate` true)
      (bind _result (`/Engine/EditorBlueprintResources/StandardMacros.IncrementInt` (`/Game/GameInstance/GI_Perso.curMissionBalise` _asgi_perso))
        (:`  `
          (set `/Game/GameInstance/GI_Perso.curMissionBalise` _result _asgi_perso)
          (`Widget.RemoveFromParent` (`self.InteractPrompt`)))))))

(event `/Game/Blueprint/BPI_Interact.TakeWhenChoiceObject`
  (cast `/Game/GameInstance/GI_Perso` (`GameplayStatics.GetGameInstance`))
  (goto _label))

(fn `UserConstructionScript`)